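; Player marine pawn that handles movement, look, aim state and cosmetic weapon firing, and creates the player HUD on BeginPlay.
; Movement follows control yaw, and turn and look-up sensitivity switch while Aim is held.
; Firing toggles the muzzle effect and a looping shot sound with an end cue.
; Any key updates gamepad detection for a deadzone-filtered mouse/thumbstick directional aim routine, which is currently never called.
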(event EventBeginPlay
  (bind _returnvalue (Game|ConstructObjectfromClass "/Game/UI/Widgets/PlayerHUD.PlayerHUD_C" (Game|Player|GetPlayerPawn 0) self))
  (UserInterface|Viewport|AddtoViewport _returnvalue 0))

(event Collision|EventActorBeginOverlap
  (params (OtherActor :type Actor%20Object%20Reference)))

(event EventTick
  (params (DeltaSeconds :type Float%20%28single-precision%29)))

(event Input|ActionEvents|InputActionFire
  (params (Key :type Key%20Structure :default "None"))
  ;[1 1 1] Fire Weapon
  (:Pressed
    (CallFunction|StartFiring))
  (:Released
    (CallFunction|StopFiring)))

(event Input|ActionEvents|InputActionAim
  (params (Key :type Key%20Structure :default "None"))
  ;[1 1 1] Aim Input
  (:Pressed
    (Variables|Combat|SetAiming true))
  (:Released
    (Variables|Combat|SetAiming false)))

(event Input|AxisEvents|InputAxisMoveForward
  (params (AxisValue :type Float%20%28single-precision%29))
  ;[1 1 1] MoveForward Input
  (CallFunction|MoveForward AxisValue))

(event Input|AxisEvents|InputAxisMoveRight
  (params (AxisValue :type Float%20%28single-precision%29))
  ;[1 1 1] MoveRight Input
  (CallFunction|MoveRight AxisValue))

(event Input|AxisEvents|InputAxisTurn
  (params (AxisValue :type Float%20%28single-precision%29))
  ;[1 1 1] Mouse Turn & Look Up
  (CallFunction|Turn AxisValue))

(event Input|AxisEvents|InputAxisLookUp
  (params (AxisValue :type Float%20%28single-precision%29))
  ;[1 1 1] Mouse Turn & Look Up
  (CallFunction|LookUp AxisValue))

(event Input|KeyboardEvents|AnyKey
  (params (Key :type Key%20Structure :default "None"))
  ;[1 1 1] Set Player Input Device
  (:Pressed
    (Variables|GamepadInput|SetIsGamepad (Class|KismetInputLibrary|KeyIsGamepadKey Key))))

(fn ConstructionScript)

(fn Aim
  (if (Variables|GamepadInput|GetIsGamepad)
    (GamepadInput|ThumbstickAim)
    (else
      (MouseInput|MouseAim))))

(fn MouseAim
  (if (MouseInput|IsMouseAboveDeadzone)
    (Pawn|SetControlRotation (Game|GetPlayerController 0) (MouseInput|GetMouseAimDirection))))

(fn GetMouseVelocity
  (bind _returnvalue (Game|GetPlayerController 0))
  (bind (_deltax _deltay) (Class|PlayerController|GetInputMouseDelta _returnvalue))
  (return (/ (Math|Vector2D|MakeVector2D _deltax _deltay) (Utilities|Time|GetWorldDeltaSeconds))))

(fn IsMouseAboveDeadzone
  (return (>= (Math|Vector2D|Vector2DLength (MouseInput|GetMouseVelocity)) (Variables|MouseInput|GetMouseDeadzone))))

(fn GetMouseAimDirection
  (bind _returnvalue (MouseInput|GetMouseVelocity))
  (return (Math|Interpolation|RInterpTo (Pawn|GetControlRotation (Game|GetPlayerController 0) :!class /Script/Engine.Controller) (Math|Rotator|MakeRotator 0.0 0.0 (Class|KismetMathLibrary|DegAtan2 (.x _returnvalue) (.y _returnvalue))) (Utilities|Time|GetWorldDeltaSeconds) (Variables|MouseInput|GetMouseInterpSpeed))))

(fn ThumbstickAim
  (if (GamepadInput|IsThumbstickAboveDeadzone)
    (Pawn|SetControlRotation (Game|GetPlayerController 0) (GamepadInput|GetThumbstickAimDirection))))

(fn IsThumbstickAboveDeadzone
  (return (>= (Math|Vector2D|Vector2DLength (Math|Vector2D|MakeVector2D (Input|AxisValues|GetGamepadAimRight) (Input|AxisValues|GetGamepadAimUp))) (Variables|GamepadInput|GetThumbstickDeadzone))))

(fn GetThumbstickAimDirection
  (return (Math|Rotator|MakeRotator 0.0 0.0 (Class|KismetMathLibrary|DegAtan2 (Input|AxisValues|GetGamepadAimUp) (Input|AxisValues|GetGamepadAimRight)))))

(fn StartFiring
  (Components|Activation|SetActive (Variables|Default|GetP_BarrelMuzzle) true false)
  (bind _returnvalue (Audio|SpawnSound2D "/Game/Sounds/Weapon_AssaultRifle/Stereo/AssaultRifle_ShotLoop_Stereo_Cue.AssaultRifle_ShotLoop_Stereo_Cue" 1.0 1.0 0.0 0 false false))
  (Variables|Default|SetWeaponFireSound _returnvalue))

(fn StopFiring
  (bind _weaponfiresound (Variables|Default|GetWeaponFireSound))
  (Components|Activation|Deactivate (Variables|Default|GetP_BarrelMuzzle))
  (Utilities|IsValid _weaponfiresound
    (:Is%20Valid
      (Audio|Components|Audio|Stop _weaponfiresound)
      (Audio|SpawnSound2D "/Game/Sounds/Weapon_AssaultRifle/Stereo/AssaultRifle_ShotEnd_Stereo_Cue.AssaultRifle_ShotEnd_Stereo_Cue" 1.0 1.0 0.0 0))))

(fn MoveForward
  (params (Value :type Float%20%28single-precision%29))
  (bind _output_get (LocalVariables|SetRotation (Pawn|GetControlRotation (Pawn|GetController) :!class /Script/Engine.Controller)))
  (LocalVariables|SetRotationYaw (Math|Rotator|MakeRotator 0.0 0.0 (.yaw _output_get)))
  (bind _output_get_2 (LocalVariables|SetDirection (.X (Math|Rotator|GetAxes (LocalVariables|GetRotationYaw)))))
  (Pawn|Input|AddMovementInput _output_get_2 Value false)
  (return))

(fn MoveRight
  (params (Value :type Float%20%28single-precision%29))
  (bind _output_get (LocalVariables|SetRotation (Pawn|GetControlRotation (Game|Player|GetPlayerPawn 0) :!class /Script/Engine.Pawn)))
  (LocalVariables|SetRotationYaw (Math|Rotator|MakeRotator 0.0 0.0 (.yaw _output_get)))
  (bind _output_get_2 (LocalVariables|SetDirection (.Y (Math|Rotator|GetAxes (LocalVariables|GetRotationYaw)))))
  (Pawn|Input|AddMovementInput _output_get_2 Value false))

(fn Turn
  (params (Value :type Float%20%28single-precision%29))
  (if (Variables|Combat|GetAiming)
    (bind _output_get (LocalVariables|SetTurnScaleFactor (Variables|Camera|GetMouseAimTurn)))
    (Pawn|Input|AddControllerYawInput (* _output_get Value))
    (else
      (bind _output_get_2 (LocalVariables|SetTurnScaleFactor (Variables|Camera|GetMouseTurn)))
      (Pawn|Input|AddControllerYawInput (* _output_get_2 Value)))))

(fn LookUp
  (params (Value :type Float%20%28single-precision%29))
  (LocalVariables|SetLookUpValue Value)
  (if (Variables|Combat|GetAiming)
    (bind _output_get (LocalVariables|SetLookUpScaleFactor (Variables|Camera|GetMouseAimLookUp)))
    (Pawn|Input|AddControllerPitchInput (* _output_get (LocalVariables|GetLookUpValue)))
    (else
      (bind _output_get_2 (LocalVariables|SetLookUpScaleFactor (Variables|Camera|GetMouseLookUp)))
      (Pawn|Input|AddControllerPitchInput (* _output_get_2 (LocalVariables|GetLookUpValue))))))